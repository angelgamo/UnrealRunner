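; Player pawn for a recoil-driven gun: each shot spends a bullet and, while ammo remains, spins and pushes it.
; Vertical thrust moves the Capsule, while horizontal thrust drives a separate Physics2 body whose velocity sets background shader speed.
; Tick makes the camera follow the Capsule, damps positive spin and updates HUD velocity.
; A delay periodically adds Physics2's X to Distance, updates the HUD and resets that body to origin.
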(event `self.ReceiveBeginPlay`
  (bind _asgmbbp (cast `/Game/BP/GMBBP` (`GameplayStatics.GetGameMode`)))
  (set `self.GMBBP` _asgmbbp)
  (`/Game/HUD.SetAmmo` (`/Game/BP/GMBBP.Hud` (`self.GMBBP`)) (`self.Bullets`)))

(event `InputAction|Shoot`
  (params (Key :type "Key Structure"))
  (:`Pressed`
    (`self.Shoot`)))

(event `self.ReceiveTick`
  (params (DeltaSeconds :type "Float (single-precision)"))
  (bind _capsule (`self.Capsule`))
  (bind _physics2 (`self.Physics2`))
  (bind _hud (`/Game/BP/GMBBP.Hud` (`self.GMBBP`)))
  (`|ExecutionSequence`
    (:`then_0`
      (`self.CameraFollow` (`self.Camera`) _capsule))
    (:`then_1`
      (`self.GunDrag` DeltaSeconds _capsule))
    (:`then_2`
      (`KismetSystemLibrary.Delay` 10.0)
      (bind _returnvalue (+ (stale _output_get) (.x (`SceneComponent.K2_GetComponentLocation` _physics2))))
      (bind _output_get (set `self.Distance` _returnvalue))
      (`/Game/HUD.SetDistance` _hud (`KismetMathLibrary.FTrunc` _returnvalue))
      (`SceneComponent.K2_SetWorldLocation` _physics2 (0.0 0.0 0.0) false true))
    (:`then_3`
      (bind _returnvalue_2 (`PrimitiveComponent.GetPhysicsLinearVelocity` _physics2 "None"))
      (bind _x (.x _returnvalue_2))
      (`/Game/HUD.SetVelocity` _hud (`KismetMathLibrary.FTrunc` _x))
      (`KismetMaterialLibrary.SetScalarParameterValue` "/Game/FondoParameters.FondoParameters" "ShaderSpeed" (`KismetMathLibrary.Lerp` -1.75 1.75 (`KismetMathLibrary.NormalizeToRange` _x -10000.0 10000.0))))))

(fn `CameraFollow`
  (params (Camera :type "CameraComponent Object Reference") (Follow :type "CapsuleComponent Object Reference"))
  (`SceneComponent.K2_SetRelativeLocation` Camera (`SceneComponent.RelativeLocation` Follow) false false))

(fn `GunDrag`
  (params (DeltaSeconds :type "Float (double-precision)") (Target :type "CapsuleComponent Object Reference"))
  (bind (_x _y) (`KismetMathLibrary.BreakVector3f` (`PrimitiveComponent.GetPhysicsAngularVelocityInDegrees` Target "None")))
  (`/Engine/EditorBlueprintResources/StandardMacros.CompareFloat` _y
    (:`>`
      (`PrimitiveComponent.SetPhysicsAngularVelocityInDegrees` Target (`KismetMathLibrary.MakeVector` 0.0 (- _y (* DeltaSeconds (`self.AngularDrag`)))) false "None"))))

(fn `Shoot`
  (bind _shootforce (`self.ShootForce`))
  (bind _capsule (`self.Capsule`))
  ;[1 0.9336 0.05524] BulletSubstract
  (bind _output_get (set `self.Bullets` (- (`self.Bullets`) 1)))
  (`/Game/HUD.SetAmmo` (`/Game/BP/GMBBP.Hud` (`self.GMBBP`)) _output_get)
  (`/Engine/EditorBlueprintResources/StandardMacros.CompareInt` _output_get
    (:`>`
      ;[0.1737 0.536 1] HandRotation
      (`PrimitiveComponent.AddForceAtLocationLocal` _capsule (`KismetMathLibrary.MakeVector` 0.0 0.0 (`self.ShootRotation`)) (`self.Offset`) "None")
      ;[1 0.2294 0.4] HandMovement
      (`PrimitiveComponent.AddForce` _capsule (`KismetMathLibrary.MakeVector` 0.0 0.0 (.z (* (`SceneComponent.GetUpVector` _capsule) (`KismetMathLibrary.MakeVector` _shootforce 0.0 _shootforce)))) "None" false)
      ;[0.4294 0.3049 1] Horizontal Physics
      (`PrimitiveComponent.AddForce` (`self.Physics2`) (`KismetMathLibrary.MakeVector` (.x (* (`SceneComponent.GetUpVector` _capsule) (`KismetMathLibrary.MakeVector` _shootforce 0.0 _shootforce)))) "None" false))))

(fn `UserConstructionScript`)