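; SpawnerAmmoBP is a spawner actor that repeatedly creates AmmoClass actors at random positions on an XZ plane.
; Tick feeds a random Delay of 0.5 to 1.5 seconds, which paces the spawns.
; Each spawn takes Y, rotation and scale from the root component, while X and Z come from scaled random unit vectors, so they center on world origin rather than the spawner.
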(event `self.ReceiveTick`
  (params (DeltaSeconds :type "Float (single-precision)"))
  (`KismetSystemLibrary.Delay` (`KismetMathLibrary.RandomFloatInRange` 0.5 1.5))
  (`|SpawnActorFromClass` (`self.AmmoClass`) (`KismetMathLibrary.MakeTransform` (`KismetMathLibrary.MakeVector` (.x (* (`KismetMathLibrary.RandomUnitVector`) (150.0 0.0 200.0))) (.y (.location (`SceneComponent.K2_GetComponentToWorld` (`self.DefaultSceneRoot`)))) (.z (* (`KismetMathLibrary.RandomUnitVector`) (150.0 0.0 200.0)))) (.rotation (`SceneComponent.K2_GetComponentToWorld` (`self.DefaultSceneRoot`))) (.scale (`SceneComponent.K2_GetComponentToWorld` (`self.DefaultSceneRoot`)))) "Undefined" "OverrideRootScale" null null))

(fn `UserConstructionScript`)